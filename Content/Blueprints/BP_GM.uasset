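; BP_GM is a Blueprint that decides when the current stage is cleared and loads the next one.
; Its CheckGame event counts actors tagged "Target" and, when none remain, prints a message and waits briefly.
; It then reads the NextStage value from the first BP_StageName actor in the level and opens that level by name.
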(event `CheckGame`
  (bind _outactors (`GameplayStatics.GetAllActorsWithTag` "Target"))
  (if (== (`KismetArrayLibrary.Array_Length` _outactors) 0)
    (`KismetSystemLibrary.PrintString` "Go To Next Stage")
    (`KismetSystemLibrary.Delay` 3.0)
    (bind _outactors_2 (`GameplayStatics.GetAllActorsOfClass` "/Game/Blueprints/BP_StageName.BP_StageName_C"))
    (`GameplayStatics.OpenLevel` (`KismetStringLibrary.Conv_StringToName` (`/Game/Blueprints/BP_StageName.NextStage` (`|GetArrayItem` _outactors_2))))))

(fn `UserConstructionScript`)