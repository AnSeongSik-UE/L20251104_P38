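; BP_Missile is a missile actor that destroys actors tagged Target when it overlaps them.
; On a hit it plays an explosion sound and particle effect, calls CheckGame on the BP_GM game mode, then destroys itself.
; A delay started at BeginPlay removes the missile after a few seconds, while a separate SetLifeSpan node is left unconnected.
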(event `self.ReceiveBeginPlay`
  (`KismetSystemLibrary.Delay` 5.0)
  (`self.K2_DestroyActor`))

(event `self.ReceiveActorBeginOverlap`
  (params (OtherActor :type "Actor Object Reference"))
  (bind _returnvalue (`self.K2_GetActorLocation`))
  (if (`self.ActorHasTag` OtherActor "Target")
    (`self.K2_DestroyActor` OtherActor)
    (`GameplayStatics.SpawnSoundAtLocation` "/Game/StarterContent/Audio/Explosion_Cue.Explosion_Cue" _returnvalue (struct) 1.0 1.0 0.0 null null)
    (`GameplayStatics.SpawnEmitterAtLocation` "/Game/StarterContent/Particles/P_Explosion.P_Explosion" _returnvalue)
    (bind _asbp_gm (cast `/Game/Blueprints/BP_GM` (`GameplayStatics.GetGameMode`)))
    (`/Game/Blueprints/BP_GM.CheckGame` _asbp_gm)
    (`self.K2_DestroyActor`)))

(fn `UserConstructionScript`)